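; BP_Functions is a shared set of helper functions for UI and camera tasks on player 0.
; CreateWidgetToViewpoint adds a widget to the viewport, then sets either UI-only input with cursor or game-only input without it.
; StartPlayerCameraFade runs a camera fade that holds when finished.
; CreateNotify spawns W_Notify through the widget helper and sets its text, also forcing game-only input and hiding the cursor.
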(fn `CreateNotify`
  (params (Text :type Text))
  (bind _returnvalue (`self.CreateWidgetToViewpoint` "/Game/Blueprints/UI/Levels/W_Notify.W_Notify_C" false (`local.__WorldContext`)))
  (bind _asw_notify (cast `/Game/Blueprints/UI/Levels/W_Notify` _returnvalue))
  (`/Game/Blueprints/UI/Levels/W_Notify.SetNotifyText` _asw_notify Text))

(fn `CreateWidgetToViewpoint`
  (params (WidgetClass :type "UserWidget Class Reference") (EnableInputUIOnly :type Boolean))
  (returns (ReturnValue :type "UserWidget Object Reference"))
  (bind _returnvalue (`GameplayStatics.GetPlayerController` (`local.__WorldContext`)))
  (bind _returnvalue_2 (`|CreateWidget` WidgetClass _returnvalue))
  (`UserWidget.AddToViewport` _returnvalue_2 0)
  (if EnableInputUIOnly
    (`WidgetBlueprintLibrary.SetInputMode_UIOnlyEx` _returnvalue _returnvalue_2)
    (set `PlayerController.bShowMouseCursor` true _returnvalue)
    (else
      (`WidgetBlueprintLibrary.SetInputMode_GameOnly` _returnvalue)
      (set `PlayerController.bShowMouseCursor` false _returnvalue)))
  (return _returnvalue_2))

(fn `StartPlayerCameraFade`
  (params (FromAlpha :type "Float (double-precision)") (ToAlpha :type "Float (double-precision)") (Duration :type "Float (double-precision)"))
  (`PlayerCameraManager.StartCameraFade` :`self` (`GameplayStatics.GetPlayerCameraManager` (`local.__WorldContext`)) :`FromAlpha` FromAlpha :`ToAlpha` ToAlpha :`Duration` Duration :`bHoldWhenFinished` true))