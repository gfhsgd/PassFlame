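; BP_GameStateLevel2 is, by its name, the game state for level 2, tracking how many curling stones have come to rest in target triggers.
; Every tick it gathers all BP_CurlingInTrigger actors and recounts those flagged IsCurlingInAndStop.
; It checks whether the count equals three, but nothing follows that branch yet, so reaching it has no effect.
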(event `self.ReceiveTick`
  (params (DeltaSeconds :type "Float (single-precision)"))
  (set `self.CurlingInStopCount` 0)
  (bind _outactors (`GameplayStatics.GetAllActorsOfClass` "/Game/Blueprints/Level2/BP_CurlingInTrigger.BP_CurlingInTrigger_C"))
  (for _array_element _outactors
    (if (`/Game/Blueprints/Level2/BP_CurlingInTrigger.IsCurlingInAndStop` _array_element)
      (set `self.CurlingInStopCount` (+ (`self.CurlingInStopCount`) 1))))
  (if (== (`self.CurlingInStopCount`) 3)
    _))

(fn `UserConstructionScript`)