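; BP_TCPClient is a TCP client that opens a connection to a local server when play begins.
; Connect and disconnect events print status messages in Chinese, and a successful connection sets IsConnect, which is not cleared on disconnect.
; Each received message is read as a string into ReceiveString, replacing the previous one.
; An unconnected loop that appends array elements and prints the result never runs.
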(event `self.ReceiveBeginPlay`
  (`self.Connect` "127.0.0.1" 3000 (delegate `OnDisconnected`) (delegate `OnConnected`) (delegate `OnMessageReceived`)))

(event `OnDisconnected`
  (params (ConnectionId :type Integer))
  (`KismetSystemLibrary.PrintString` "连接已断开"))

(event `OnConnected`
  (params (ConnectionId :type Integer))
  (`KismetSystemLibrary.PrintString` "连接成功")
  (set `self.IsConnect` true))

(event `OnMessageReceived`
  (params (ConnectionId :type Integer) (Message :type "Array of Byte (by ref)"))
  (bind _returnvalue (`self.Message_ReadString` Message (`KismetArrayLibrary.Array_Length` Message)))
  (set `self.ReceiveString` _returnvalue))

(fn `UserConstructionScript`)