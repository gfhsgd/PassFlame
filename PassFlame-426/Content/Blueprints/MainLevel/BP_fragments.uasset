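; Collectible sport-fragment pickup that counts toward unlocking Winter Olympic sports in the illustrated-guide (codex) system.
; AttachField overlap by the main character plays a timeline that shrinks the fragment and pulls it toward the player, showing a tutorial tip if none has been collected before.
; Box overlap decrements the GameInstance fragment count keyed by the actor's first tag, shows a notification, sets HasMeetFragment and destroys the actor.
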(event `self.AttachField.OnComponentBeginOverlap`
  (params (OverlappedComponent :type "PrimitiveComponent Object Reference") (OtherActor :type "Actor Object Reference") (OtherComp :type "PrimitiveComponent Object Reference") (OtherBodyIndex :type Integer) (bFromSweep :type Boolean) (SweepResult :type "HitResult Structure (by ref)"))
  (bind _alpha (`self.Alpha`))
  (cast `/Game/Blueprints/BP_MainCharacter` OtherActor)
  (`|ExecutionSequence`
    (:`then_0`
      (if (not (`/Game/Blueprints/GameBase/BP_GameInstance.HasMeetFragment` (cast `/Game/Blueprints/GameBase/BP_GameInstance` (`GameplayStatics.GetGameInstance`) :!pure true)))
        (`/Engine/EditorBlueprintResources/StandardMacros.DoOnce` false
          (:`Completed`
            (bind _returnvalue (`/Game/Blueprints/GameBase/BP_Functions.CreateWidgetToViewpoint` "/Game/Blueprints/UI/Levels/W_Tips.W_Tips_C"))
            (bind _asw_tips (cast `/Game/Blueprints/UI/Levels/W_Tips` _returnvalue))
            (`/Game/Blueprints/UI/Levels/W_Tips.SetTipText` _asw_tips "遇到了运动碎片，收集后可在图鉴系统中解锁对应的冬奥会运动哦！")))))
    (:`then_1`
      (set `self.InitialLocation` (`self.K2_GetActorLocation`))
      (set `self.InitialScale` (`self.GetActorScale3D`))
      (bind (_direction _alpha_2) (`Timeline|Timeline`)
        (:`Update`
          (set `self.Alpha` _alpha_2)
          (`self.K2_SetActorLocation` (`KismetMathLibrary.VLerp` (`self.InitialLocation`) (`self.K2_GetActorLocation` (`GameplayStatics.GetPlayerCharacter` 0)) _alpha))
          (`self.SetActorScale3D` (`KismetMathLibrary.VLerp` (`self.InitialScale`) (0.0 0.0 0.0) _alpha)))))))

(event `self.Box.OnComponentBeginOverlap`
  (params (OverlappedComponent :type "PrimitiveComponent Object Reference") (OtherActor :type "Actor Object Reference") (OtherComp :type "PrimitiveComponent Object Reference") (OtherBodyIndex :type Integer) (bFromSweep :type Boolean) (SweepResult :type "HitResult Structure (by ref)"))
  (cast `/Game/Blueprints/BP_MainCharacter` OtherActor)
  (`/Game/Blueprints/GameBase/BP_GameInstance.MinusFragmentsCount` (cast `/Game/Blueprints/GameBase/BP_GameInstance` (`GameplayStatics.GetGameInstance`) :!pure true) (`|GetArrayItem` (`self.Tags`)))
  (bind _returnvalue (`/Game/Blueprints/GameBase/BP_Functions.CreateWidgetToViewpoint` "/Game/Blueprints/UI/Levels/W_Notify.W_Notify_C"))
  (bind _asw_notify (cast `/Game/Blueprints/UI/Levels/W_Notify` _returnvalue))
  (`/Game/Blueprints/UI/Levels/W_Notify.SetNotifyText` _asw_notify "图鉴碎片+1")
  (set `/Game/Blueprints/GameBase/BP_GameInstance.HasMeetFragment` true (cast `/Game/Blueprints/GameBase/BP_GameInstance` (`GameplayStatics.GetGameInstance`) :!pure true))
  (`self.K2_DestroyActor`))

(fn `UserConstructionScript`)