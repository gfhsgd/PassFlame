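; BP_SlideWayInitial is a slide trigger that puts BP_MainCharacter into skiing mode while inside its SkiBox.
; The first entry plays switch effects and snow audio, then sets the player's IsSkiing flag and snowboard state; the first exit clears both.
; While InCollision is set, Tick pushes the player along their forward vector through movement input.
; Each overlap handler has a DoOnce that is never reset, so each transition fires only once.
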(event `self.SkiBox.OnComponentBeginOverlap`
  (params (OverlappedComponent :type "PrimitiveComponent Object Reference") (OtherActor :type "Actor Object Reference") (OtherComp :type "PrimitiveComponent Object Reference") (OtherBodyIndex :type Integer) (bFromSweep :type Boolean) (SweepResult :type "HitResult Structure (by ref)"))
  (bind _asbp_main_character (cast `/Game/Blueprints/BP_MainCharacter` (`GameplayStatics.GetPlayerCharacter` 0) :!pure true))
  (cast `/Game/Blueprints/BP_MainCharacter` OtherActor)
  (`/Engine/EditorBlueprintResources/StandardMacros.DoOnce` false
    (:`Completed`
      ;[1 1 1] 声音特效
      (`GameplayStatics.SpawnEmitterAttached` "/Game/CartoonyFXPACK4/Particles/AnimeFX/HandDrawn/P_SwitchState.P_SwitchState" (`Actor.RootComponent` (`GameplayStatics.GetPlayerCharacter` 0)) "None" (0.0 0.0 0.0) (struct) (1.0 1.0 1.0) "SnapToTarget")
      (`GameplayStatics.PlaySound2D` "/Game/Audios/Au_SwitchState.Au_SwitchState" 1.0 1.0 0.0 null null)
      (`GameplayStatics.PlaySound2D` "/Game/Audios/Snow_Cue.Snow_Cue" 1.0 1.0 1.0 null null false)
      (set `self.InCollision` true)
      (set `/Game/Blueprints/BP_MainCharacter.IsSkiing` true _asbp_main_character)
      (`/Game/Blueprints/BP_MainCharacter.SetSnowBoard` _asbp_main_character true))))

(event `self.SkiBox.OnComponentEndOverlap`
  (params (OverlappedComponent :type "PrimitiveComponent Object Reference") (OtherActor :type "Actor Object Reference") (OtherComp :type "PrimitiveComponent Object Reference") (OtherBodyIndex :type Integer))
  (bind _asbp_main_character (cast `/Game/Blueprints/BP_MainCharacter` (`GameplayStatics.GetPlayerCharacter` 0) :!pure true))
  (cast `/Game/Blueprints/BP_MainCharacter` OtherActor)
  (`/Engine/EditorBlueprintResources/StandardMacros.DoOnce` false
    (:`Completed`
      (set `self.InCollision` false)
      (set `/Game/Blueprints/BP_MainCharacter.IsSkiing` false _asbp_main_character)
      (`/Game/Blueprints/BP_MainCharacter.SetSnowBoard` _asbp_main_character false))))

(event `self.ReceiveTick`
  (params (DeltaSeconds :type "Float (single-precision)"))
  (bind _returnvalue (`GameplayStatics.GetPlayerCharacter` 0))
  (if (`self.InCollision`)
    (`Pawn.AddMovementInput` _returnvalue (`self.GetActorForwardVector` _returnvalue) 1.5 false)))

(fn `UserConstructionScript`)