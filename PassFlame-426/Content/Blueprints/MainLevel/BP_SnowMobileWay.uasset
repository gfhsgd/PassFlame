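; BP_SnowMobileWay is a trigger zone that puts the player character into snowmobile mode while inside its box.
; On overlap it plays switch effects, sets the character's snowmobile state and raises or changes walk speed to SnowMobileVelocity.
; While overlapped, Tick pushes the player forward along its facing.
; On exit it restores normal speed and state only if no other SnowMobileWay instance still contains the player, so adjoining zones chain seamlessly.
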(event `self.Box.OnComponentBeginOverlap`
  (params (OverlappedComponent :type "PrimitiveComponent Object Reference") (OtherActor :type "Actor Object Reference") (OtherComp :type "PrimitiveComponent Object Reference") (OtherBodyIndex :type Integer) (bFromSweep :type Boolean) (SweepResult :type "HitResult Structure (by ref)"))
  (bind _asbp_main_character (cast `/Game/Blueprints/BP_MainCharacter` (`GameplayStatics.GetPlayerCharacter` 0) :!pure true))
  (cast `/Game/Blueprints/BP_MainCharacter` OtherActor)
  (set `self.InCollision` true)
  ;[1 1 1] 声音和特效
  (`GameplayStatics.SpawnEmitterAttached` "/Game/CartoonyFXPACK4/Particles/AnimeFX/HandDrawn/P_SwitchState.P_SwitchState" (`Actor.RootComponent` (`GameplayStatics.GetPlayerCharacter` 0)) "None" (0.0 0.0 0.0) (struct) (1.0 1.0 1.0) "SnapToTarget")
  (`GameplayStatics.PlaySound2D` "/Game/Audios/Au_SwitchState.Au_SwitchState" 1.0 1.0 0.0 null null)
  (set `/Game/Blueprints/BP_MainCharacter.IsInSnowMoblie` true _asbp_main_character)
  (`/Game/Blueprints/BP_MainCharacter.SetSnowMobile` _asbp_main_character true)
  (set `CharacterMovementComponent.MaxWalkSpeed` (`self.SnowMobileVelocity`) (`Character.CharacterMovement` _asbp_main_character)))

(event `self.Box.OnComponentEndOverlap`
  (params (OverlappedComponent :type "PrimitiveComponent Object Reference") (OtherActor :type "Actor Object Reference") (OtherComp :type "PrimitiveComponent Object Reference") (OtherBodyIndex :type Integer))
  (bind _asbp_main_character (cast `/Game/Blueprints/BP_MainCharacter` (`GameplayStatics.GetPlayerCharacter` 0) :!pure true))
  (cast `/Game/Blueprints/BP_MainCharacter` OtherActor)
  (set `self.InCollision` false)
  (if (not (`self.IsPlayerInOtherSnowMobileWay`))
    (set `/Game/Blueprints/BP_MainCharacter.IsInSnowMoblie` false _asbp_main_character)
    (`/Game/Blueprints/BP_MainCharacter.SetSnowMobile` _asbp_main_character false)
    (set `CharacterMovementComponent.MaxWalkSpeed` 600.0 (`Character.CharacterMovement` _asbp_main_character))))

(event `self.ReceiveTick`
  (params (DeltaSeconds :type "Float (single-precision)"))
  (bind _returnvalue (`GameplayStatics.GetPlayerCharacter` 0))
  (if (`self.InCollision`)
    (`Pawn.AddMovementInput` _returnvalue (`self.GetActorForwardVector` _returnvalue) 1.0 false)))

(fn `IsPlayerInOtherSnowMobileWay`
  (returns (return :type Boolean))
  (bind _outactors (`GameplayStatics.GetAllActorsOfClass` "BP_SnowMobileWay_C"))
  (for _array_element _outactors
    (if (`/Game/Blueprints/MainLevel/BP_SnowMobileWay.InCollision` _array_element)
      (return true)))
  (return false))

(fn `UserConstructionScript`)