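; Level gate actor that carries the player from the main level into a new level.
; Its first actor tag is the level number, compared with GameInstance's MaxLevelOpened to start already-unlocked doors swung open.
; Character overlap shows a first-time tip and, for locked doors, plays a one-shot timeline opening both leaves.
; It then saves the player's spawn transform and progress, fades out, shows a loading widget and opens LevelToOpen after fixed delays.
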(event `self.ReceiveBeginPlay`
  (if (<= (`KismetStringLibrary.Conv_StringToInt` (`KismetStringLibrary.Conv_NameToString` (`|GetArrayItem` (`self.Tags`)))) (`/Game/Blueprints/GameBase/BP_GameInstance.MaxLevelOpened` (cast `/Game/Blueprints/GameBase/BP_GameInstance` (`GameplayStatics.GetGameInstance`) :!pure true)))
    (`SceneComponent.K2_AddLocalRotation` (`self.DoorL`) (struct :`Yaw` 90.0) false false)
    (`SceneComponent.K2_AddLocalRotation` (`self.DoorR`) (struct :`Yaw` -90.0) false false)))

(event `self.Box.OnComponentBeginOverlap`
  (params (OverlappedComponent :type "PrimitiveComponent Object Reference") (OtherActor :type "Actor Object Reference") (OtherComp :type "PrimitiveComponent Object Reference") (OtherBodyIndex :type Integer) (bFromSweep :type Boolean) (SweepResult :type "HitResult Structure (by ref)"))
  (bind _asbp_game_instance (cast `/Game/Blueprints/GameBase/BP_GameInstance` (`GameplayStatics.GetGameInstance`) :!pure true))
  (cast `/Game/Blueprints/BP_MainCharacter` OtherActor)
  (`|ExecutionSequence`
    (:`then_0`
      (if (not (`/Game/Blueprints/GameBase/BP_GameInstance.HasMeetLevelDoor` (cast `/Game/Blueprints/GameBase/BP_GameInstance` (`GameplayStatics.GetGameInstance`) :!pure true)))
        (bind _returnvalue (`/Game/Blueprints/GameBase/BP_Functions.CreateWidgetToViewpoint` "/Game/Blueprints/UI/Levels/W_Tips.W_Tips_C"))
        (bind _asw_tips (cast `/Game/Blueprints/UI/Levels/W_Tips` _returnvalue))
        (`/Game/Blueprints/UI/Levels/W_Tips.SetTipText` _asw_tips "关卡之门会将你带到一个全新的世界，你将在其中继续你的火炬传递之旅！")))
    (:`then_1`
      (if (> (`KismetStringLibrary.Conv_StringToInt` (`KismetStringLibrary.Conv_NameToString` (`|GetArrayItem` (`self.Tags`)))) (`/Game/Blueprints/GameBase/BP_GameInstance.MaxLevelOpened` (cast `/Game/Blueprints/GameBase/BP_GameInstance` (`GameplayStatics.GetGameInstance`) :!pure true)))
        (`/Engine/EditorBlueprintResources/StandardMacros.DoOnce` false
          (:`Completed`
            (`GameplayStatics.PlaySound2D` "/Game/Audios/Au_OpenTheDoor.Au_OpenTheDoor" 1.0 1.0 0.0 null null false)
            (bind (_direction _ldoorrotation _rdoorrotation) (`Timeline|OpenDoorTimeLine`)
              (:`Update`
                (`SceneComponent.K2_AddLocalRotation` (`self.DoorL`) (`KismetMathLibrary.MakeRotator` 0.0 0.0 _ldoorrotation) false false)
                (`SceneComponent.K2_AddLocalRotation` (`self.DoorR`) (`KismetMathLibrary.MakeRotator` 0.0 0.0 _rdoorrotation) false false))
              (:`Finished`
                (`/Game/Blueprints/GameBase/BP_GameInstance.SetPlayerSpawnTransform` _asbp_game_instance (`self.GetTransform` (`GameplayStatics.GetPlayerCharacter` 0)))
                (set `/Game/Blueprints/GameBase/BP_GameInstance.MaxLevelOpened` (+ (`/Game/Blueprints/GameBase/BP_GameInstance.MaxLevelOpened` _asbp_game_instance) 1) _asbp_game_instance)
                (set `/Game/Blueprints/GameBase/BP_GameInstance.HasMeetLevelDoor` true (cast `/Game/Blueprints/GameBase/BP_GameInstance` (`GameplayStatics.GetGameInstance`) :!pure true))
                (`KismetSystemLibrary.Delay` 0.2)
                (`PlayerCameraManager.StartCameraFade` :`self` (`GameplayStatics.GetPlayerCameraManager` 0) :`ToAlpha` 1.0 :`Duration` 1.0 :`bHoldWhenFinished` true)
                (`KismetSystemLibrary.Delay` 1.0)
                (`WidgetLayoutLibrary.RemoveAllWidgets`)
                ;[1 1 1] 进入加载界面
                (bind _returnvalue_2 (`/Game/Blueprints/GameBase/BP_Functions.CreateWidgetToViewpoint` "/Game/Blueprints/UI/UILevel/W_Loading.W_Loading_C"))
                (bind _asw_loading (cast `/Game/Blueprints/UI/UILevel/W_Loading` _returnvalue_2))
                (set `/Game/Blueprints/UI/UILevel/W_Loading.LoopMax` 2 _asw_loading)
                (`KismetSystemLibrary.Delay` 8.0)
                (`GameplayStatics.OpenLevelBySoftObjectPtr` (`self.LevelToOpen`))))))))))

(fn `UserConstructionScript`)